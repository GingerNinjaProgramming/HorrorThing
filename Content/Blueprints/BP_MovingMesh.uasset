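; BP_MovingMesh is an actor that jumps to a preset transform, once, when something leaves its linked TriggerBox.
; The end-overlap event teleports the actor to NewTransform without sweep and plays MoveSound at that location.
; It then destroys the TriggerBox so the move cannot repeat.
; A forward debug line trace is left in the graph but never runs.
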(event `self.ReceiveTick`
  (params (DeltaSeconds :type "Float (single-precision)")))

(event `self.TriggerBox.OnActorEndOverlap`
  (params (OverlappedActor :type "Actor Object Reference") (OtherActor :type "Actor Object Reference"))
  (bind _newtransform (`self.NewTransform`))
  (if (`KismetSystemLibrary.IsValid` (`self.TriggerBox`))
    (`self.K2_SetActorTransform` _newtransform false true)
    (`GameplayStatics.PlaySoundAtLocation` (`self.MoveSound`) (.location _newtransform) (struct) 1.0 1.0 0.0 null null null null)
    (`self.K2_DestroyActor` (`self.TriggerBox`))))

(fn `UserConstructionScript`)