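; BP_WPAngel is a Weeping Angel-style AI character that advances on the player while unseen and freezes when watched.
; Each tick, a dot product checks whether the player faces it, then a camera-to-head visibility trace detects blockers.
; It stops immediately when faced with a clear trace, otherwise it uses AI MoveTo toward the player.
; When the player overlaps its box, it snaps their control yaw toward itself.
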(event `self.ReceiveBeginPlay`
  (bind _asbp_first_person_character (cast `/Game/Blueprints/Player/BP_FirstPersonCharacter` (`GameplayStatics.GetPlayerCharacter` 0)))
  (set `self.PlayerRef` _asbp_first_person_character))

(event `self.ReceiveTick`
  (params (DeltaSeconds :type "Float (single-precision)"))
  (bind _playerref (`self.PlayerRef`))
  (if (> (`KismetMathLibrary.Dot_VectorVector` (`KismetMathLibrary.Normal` (- (`self.K2_GetActorLocation`) (`self.K2_GetActorLocation` _playerref))) (`self.GetActorForwardVector` _playerref)) 0.7)
    (bind (_outhit _returnvalue) (`KismetSystemLibrary.LineTraceSingle` :`Start` (`self.K2_GetActorLocation` (`/Game/Blueprints/Player/BP_FirstPersonCharacter.GetCamera` _playerref)) :`End` (`SceneComponent.GetSocketLocation` (`self.Mesh`) "head") :`TraceChannel` "TraceTypeQuery1" :`DrawDebugType` "ForOneFrame"))
    (if _returnvalue
      (`|AIMoveTo` self (0.0 0.0 0.0) (`self.PlayerRef`) :!label _label)
      (else
        (`MovementComponent.StopMovementImmediately` (`self.CharacterMovement`))))
    (else
      (goto _label))))

(event `self.Box.OnComponentBeginOverlap`
  (params (OverlappedComponent :type "PrimitiveComponent Object Reference") (OtherActor :type "Actor Object Reference") (OtherComp :type "PrimitiveComponent Object Reference") (OtherBodyIndex :type Integer) (bFromSweep :type Boolean) (SweepResult :type "HitResult Structure (by ref)"))
  (bind _returnvalue (`GameplayStatics.GetPlayerController` 0))
  (if (== OtherActor (`GameplayStatics.GetPlayerCharacter` 0))
    (`Controller.SetControlRotation` _returnvalue (`KismetMathLibrary.MakeRotator` 0.0 0.0 (.yaw (`KismetMathLibrary.FindLookAtRotation` (`self.K2_GetActorLocation` _returnvalue) (`self.K2_GetActorLocation`)))))))

(fn `UserConstructionScript`)