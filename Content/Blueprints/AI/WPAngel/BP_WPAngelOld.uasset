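; Weeping-angel style enemy that chases the first-person player unless caught in their flashlight.
; Each tick it runs AI MoveTo unless the player's spotlight is on, the player's line-of-sight check passes and a light trace hits.
; When caught it stops and takes a random pose, with paired DoOnce gates switching between frozen and looping walk.
; Box overlap snaps the player's view yaw toward it; debug print and trace remain on.
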(event `self.ReceiveBeginPlay`
  (`|ExecutionSequence`
    (:`then_0`
      (bind _asbp_first_person_character (cast `/Game/Blueprints/Player/BP_FirstPersonCharacter` (`GameplayStatics.GetPlayerCharacter` 0)))
      (set `self.PlayerRef` _asbp_first_person_character))
    (:`then_1`
      (`SkeletalMeshComponent.PlayAnimation` (`self.Mesh`) "/Game/Static/Assets/Charecter/WPA_Mannequin/Anims/Walking.Walking" true))))

(event `self.ReceiveTick`
  (params (DeltaSeconds :type "Float (single-precision)"))
  (bind _playerref (`self.PlayerRef`))
  (if (`SceneComponent.bVisible` (`/Game/Blueprints/Player/BP_FirstPersonCharacter.SpotLight` _playerref))
    (if (> (`KismetMathLibrary.Dot_VectorVector` (`KismetMathLibrary.Normal` (- (`self.K2_GetActorLocation`) (`self.K2_GetActorLocation` _playerref))) (`self.GetActorForwardVector` _playerref)) 0.7)
      (bind (_outhit _returnvalue) (`/Game/Blueprints/BPFL_HelperLibary.Line Trace By Light` (`/Game/Blueprints/Player/BP_FirstPersonCharacter.SpotLight` _playerref) true))
      (if (not _returnvalue)
        _
        (else
          (`/Engine/EditorBlueprintResources/StandardMacros.DoOnce` false :!label _label
            (:`Completed`
              (`MovementComponent.StopMovementImmediately` (`self.CharacterMovement`))
              (`SkeletalMeshComponent.PlayAnimation` (`self.Mesh`) (`KismetArrayLibrary.Array_Random` (`self.AnimPoses`)) true)
              (goto _label_2 :!via `Reset`)))))))
  (`KismetSystemLibrary.PrintString` "\"MoveingW\"")
  (`|ExecutionSequence`
    (:`then_0`
      (`|AIMoveTo` self (0.0 0.0 0.0) (`self.PlayerRef`)
        (:`then`
          (goto _label :!via `Reset`))))
    (:`then_1`
      (`/Engine/EditorBlueprintResources/StandardMacros.DoOnce` false :!label _label_2
        (:`Completed`
          (`SkeletalMeshComponent.PlayAnimation` (`self.Mesh`) "/Game/Static/Assets/Charecter/WPA_Mannequin/Anims/Walking.Walking" true))))))

(event `self.Box.OnComponentBeginOverlap`
  (params (OverlappedComponent :type "PrimitiveComponent Object Reference") (OtherActor :type "Actor Object Reference") (OtherComp :type "PrimitiveComponent Object Reference") (OtherBodyIndex :type Integer) (bFromSweep :type Boolean) (SweepResult :type "HitResult Structure (by ref)"))
  (bind _returnvalue (`GameplayStatics.GetPlayerController` 0))
  (if (== OtherActor (`GameplayStatics.GetPlayerCharacter` 0))
    (`Controller.SetControlRotation` _returnvalue (`KismetMathLibrary.MakeRotator` 0.0 0.0 (.yaw (`KismetMathLibrary.FindLookAtRotation` (`self.K2_GetActorLocation` _returnvalue) (`self.K2_GetActorLocation`)))))))

(fn `UserConstructionScript`)