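; AI controller for NPCs that runs the BT_NPC behavior tree and tracks the player by sight.
; Perception updates feed HandleSight, which ignores everything except sight stimuli from player character 0.
; It writes the player to the TargetActor blackboard key while sensed and clears it when sight is lost, saving the stimulus position as LastKnownLocation.
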(event `self.AIPerception.OnTargetPerceptionUpdated`
  (params (Actor :type "Actor Object Reference") (Stimulus :type "AIStimulus Structure"))
  (`self.HandleSight` Actor Stimulus))

(event `self.ReceiveBeginPlay`
  (`self.RunBehaviorTree` "/Game/Blueprints/AI/BT_NPC.BT_NPC"))

(fn `HandleSight`
  (params (Actor :type "Actor Object Reference") (Stimulus :type "AIStimulus Structure (by ref)"))
  (bind (_age _expirationage _strength _stimuluslocation _receiverlocation _tag _bsuccessfullysensed) (break `AIStimulus` Stimulus))
  (bind _returnvalue (`GameplayStatics.GetPlayerCharacter` 0))
  (bind _blackboard (`self.Blackboard`))
  (bind _returnvalue_2 (`AIPerceptionSystem.GetSenseClassForStimulus` Stimulus))
  (if (and (== _returnvalue_2 "/Script/AIModule.AISense_Sight") (== Actor _returnvalue))
    (`BlackboardComponent.SetValueAsObject` _blackboard "TargetActor" (`KismetMathLibrary.SelectObject` _returnvalue null _bsuccessfullysensed))
    (if (not _bsuccessfullysensed)
      (`BlackboardComponent.SetValueAsVector` _blackboard "LastKnownLocation" _stimuluslocation))
    (else
      (return))))

(fn `UserConstructionScript`)