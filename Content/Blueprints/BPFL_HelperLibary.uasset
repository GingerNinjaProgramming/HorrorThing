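; Blueprint function library of world-context helpers for light tracing, facing checks and AI-audible sound.
; Light helpers trace the Visibility channel from a light along its forward vector to its attenuation radius, with optional debug drawing.
; IsActorInVision compares a forward dot product against VisionRange, checking angle only, not distance or occlusion.
; PlaySoundAI spawns a sound at a location and reports a noise event there, using its volume multiplier as loudness.
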(fn `GetLightReach`
  (params (Light :type "LocalLightComponent Object Reference"))
  (returns (ReturnValue :type "Vector Structure"))
  (return (+ (`SceneComponent.K2_GetComponentLocation` Light) (* (`SceneComponent.GetForwardVector` Light) (`LocalLightComponent.AttenuationRadius` Light)))))

(fn `IsActorInVision`
  (params (Actor :type "Actor Object Reference") (TargetActor :type "Actor Object Reference") (VisionRange :type "Float (double-precision)"))
  (returns (`Return Value` :type Boolean))
  (return (and (> (`KismetMathLibrary.Dot_VectorVector` (`KismetMathLibrary.Normal` (- (`Actor.K2_GetActorLocation` TargetActor) (`Actor.K2_GetActorLocation` Actor))) (`Actor.GetActorForwardVector` Actor)) VisionRange) true)))

(fn `Line Trace By Light`
  (params (Light :type "LocalLightComponent Object Reference") (IsDebug :type Boolean))
  (returns (OutHit :type "HitResult Structure") (ReturnValue :type Boolean))
  (bind (_outhit _returnvalue) (`KismetSystemLibrary.LineTraceSingle` :`WorldContextObject` (`local.__WorldContext`) :`Start` (`SceneComponent.K2_GetComponentLocation` Light) :`End` (`self.GetLightReach` Light (`local.__WorldContext`)) :`TraceChannel` "TraceTypeQuery1" :`DrawDebugType` (select `bool` IsDebug :`true` "Persistent" :!type "EDrawDebugTrace Enum")))
  (return _outhit _returnvalue))

(fn `PlaySoundAI`
  (params (SoundMaker :type "Actor Object Reference") (Sound :type "SoundBase Object Reference") (SoundLocation :type "Vector Structure") (OneShot :type Boolean :default true))
  (returns (DoesSoundExist :type Boolean) (ReturnSound :type "AudioComponent Object Reference"))
  (bind _returnvalue (`GameplayStatics.SpawnSoundAtLocation` (`local.__WorldContext`) Sound SoundLocation (struct) 1.0 1.0 0.0 null null OneShot))
  (`AISense_Hearing.ReportNoiseEvent` (`local.__WorldContext`) SoundLocation (`AudioComponent.VolumeMultiplier` _returnvalue) SoundMaker)
  (return (not (`local.OneShot`)) _returnvalue))