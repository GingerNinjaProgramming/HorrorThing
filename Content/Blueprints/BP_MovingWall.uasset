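; BP_MovingWall is a wall actor that jumps to a new position when an actor leaves its referenced trigger box.
; On end overlap, it teleports to the trigger's X and Y, keeping its height, roll, pitch and scale but zeroing yaw.
; It plays a metallic twang there and destroys the trigger, making the move one-shot.
; A forward debug line trace is left unconnected.
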(event `self.ReceiveTick`
  (params (DeltaSeconds :type "Float (single-precision)")))

(event `self.TriggerBox.OnActorEndOverlap`
  (params (OverlappedActor :type "Actor Object Reference") (OtherActor :type "Actor Object Reference"))
  (bind (_returnvalue_x _returnvalue_y) (`KismetMathLibrary.BreakVector` (`self.K2_GetActorLocation` (`self.TriggerBox`))))
  (bind _returnvalue (`KismetMathLibrary.MakeVector` _returnvalue_x _returnvalue_y (.z (.location (`self.GetTransform`)))))
  (if (`KismetSystemLibrary.IsValid` (`self.TriggerBox`))
    (`self.K2_SetActorTransform` (`KismetMathLibrary.MakeTransform` _returnvalue (`KismetMathLibrary.MakeRotator` (.roll (.rotation (`self.GetTransform`))) (.pitch (.rotation (`self.GetTransform`)))) (.scale (`self.GetTransform`))) false true)
    (`GameplayStatics.PlaySoundAtLocation` "/Game/Static/HorrorSFX/Stingers_and_Spooky_Triggers/Metal_twang.Metal_twang" _returnvalue (struct) 1.0 1.0 0.0 null null null null)
    (`self.K2_DestroyActor` (`self.TriggerBox`))))

(fn `UserConstructionScript`)