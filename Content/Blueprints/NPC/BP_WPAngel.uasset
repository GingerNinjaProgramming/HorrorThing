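; BP_WPAngel is a weeping-angel style NPC that chases the player except while being watched.
; Each tick, a dot product against the player's forward vector tests whether it is roughly in front, then a visibility trace targets its head socket.
; It stops when in front with an unblocked trace, otherwise it uses AI MoveTo toward the player.
; Overlapping its box snaps the player's control yaw to face the angel.
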(event `self.ReceiveBeginPlay`
  (bind _asbp_first_person_character (cast `/Game/FirstPerson/Blueprints/BP_FirstPersonCharacter` (`GameplayStatics.GetPlayerPawn` 0)))
  (set `self.PlayerRef` _asbp_first_person_character))

(event `self.ReceiveTick`
  (params (DeltaSeconds :type "Float (single-precision)"))
  (bind _playerref (`self.PlayerRef`))
  (bind _returnvalue (`KismetMathLibrary.Dot_VectorVector` (`KismetMathLibrary.Normal` (- (`self.K2_GetActorLocation`) (`self.K2_GetActorLocation` _playerref))) (`self.GetActorForwardVector` _playerref)))
  (`KismetSystemLibrary.PrintString` (`KismetStringLibrary.Conv_DoubleToString` _returnvalue))
  (if (> _returnvalue 0.7)
    (bind (_outhit _returnvalue_2) (`KismetSystemLibrary.LineTraceSingle` :`Start` (`self.K2_GetActorLocation` (`/Game/FirstPerson/Blueprints/BP_FirstPersonCharacter.GetCamera` _playerref)) :`End` (`SceneComponent.GetSocketLocation` (`self.Mesh`) "head") :`TraceChannel` "TraceTypeQuery1" :`DrawDebugType` "ForOneFrame"))
    (if _returnvalue_2
      (`|AIMoveTo` self (0.0 0.0 0.0) (`self.PlayerRef`) :!label _label)
      (else
        (`MovementComponent.StopMovementImmediately` (`self.CharacterMovement`))))
    (else
      (goto _label))))

(event `self.Box.OnComponentBeginOverlap`
  (params (OverlappedComponent :type "PrimitiveComponent Object Reference") (OtherActor :type "Actor Object Reference") (OtherComp :type "PrimitiveComponent Object Reference") (OtherBodyIndex :type Integer) (bFromSweep :type Boolean) (SweepResult :type "HitResult Structure (by ref)"))
  (bind _returnvalue (`GameplayStatics.GetPlayerController` 0))
  (if (== OtherActor (`GameplayStatics.GetPlayerCharacter` 0))
    (`Controller.SetControlRotation` _returnvalue (`KismetMathLibrary.MakeRotator` 0.0 0.0 (.yaw (`KismetMathLibrary.FindLookAtRotation` (`self.K2_GetActorLocation` _returnvalue) (`self.K2_GetActorLocation`)))))))

(fn `UserConstructionScript`)