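; BP_PickupTrap is an interactable pickup that toggles a set of disappearing platforms when a player interacts with it.
; Interact runs the parent behavior, calls ToggleStaticMesh on each entry in the DissaperingPlatform array, then destroys the pickup, so it fires only once.
; ToggleStaticMesh flips each mesh's visibility and sets collision to match, so hidden platforms become non-solid and hidden ones that reappear become solid.
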(event `/Game/Blueprints/Interface/BPI_Interactable.Interact`
  (params (Player :type "/Game/Blueprints/Player/BP_FirstPersonCharacter Object Reference"))
  (`parent.Interact` Player)
  (for _array_element (`self.Dissapering Platform`)
    (`self.ToggleStaticMesh` _array_element))
  (`self.K2_DestroyActor`))

(fn `ToggleStaticMesh`
  (params (Mesh :type "StaticMeshActor Object Reference"))
  (bind _staticmeshcomponent (`StaticMeshActor.StaticMeshComponent` Mesh))
  (bind _returnvalue (`SceneComponent.IsVisible` _staticmeshcomponent))
  (`SceneComponent.SetVisibility` _staticmeshcomponent (select `bool` _returnvalue :`false` true) false)
  (`PrimitiveComponent.SetCollisionEnabled` _staticmeshcomponent (select `bool` _returnvalue :`false` "NoCollision" :`true` "QueryAndPhysics" :!type "ECollisionEnabled Enum")))

(fn `UserConstructionScript`
  (`parent.UserConstructionScript`))