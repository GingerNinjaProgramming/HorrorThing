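; BP_Door is an interactable door that swings open with a squeaky sound when a player interacts with it while it is not yet open.
; A dot product of the Frame's forward vector and the player-to-frame direction picks the swing direction from the player's side.
; A timeline lerps the Door's relative yaw to a quarter turn, then sets IsDoorOpen, with no closing logic.
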(event `/Game/Blueprints/Interface/BPI_Interactable.Interact`
  (params (Player :type "/Game/Blueprints/Player/BP_FirstPersonCharacter Object Reference"))
  (bind _frame (`self.Frame`))
  (if (not (`self.IsDoorOpen`))
    (`GameplayStatics.PlaySoundAtLocation` "/Game/Static/HorrorSFX/House___Office/Door_squeeky_2.Door_squeeky_2" (`SceneComponent.K2_GetComponentLocation` (`self.Door`)) (struct) 1.0 1.0 0.0 null null null null)
    (bind _returnvalue (`KismetMathLibrary.SelectFloat` 90.0 -90.0 (not (>= (`KismetMathLibrary.Dot_VectorVector` (`SceneComponent.GetForwardVector` _frame) (`KismetMathLibrary.Normal` (- (`SceneComponent.K2_GetComponentLocation` _frame) (`self.K2_GetActorLocation` Player)))) 0.0))))
    (bind (_direction _door_float) (`Timeline|OpenDoorTimeline`)
      (:`Update`
        (`SceneComponent.K2_SetRelativeRotation` (`self.Door`) (`KismetMathLibrary.MakeRotator` 0.0 0.0 (`KismetMathLibrary.Lerp` 0.0 _returnvalue _door_float)) false false))
      (:`Finished`
        (set `self.IsDoorOpen` true)))))

(fn `UserConstructionScript`)